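; Touch-enabled grid tile for what appears to be path-based player movement.
; On Tick, after a two-second Delay, it shows its Over mesh with an orange texture via a dynamic material; touch enter only prints hit coordinates.
; Disconnected logic would append positions to ActorForTestingThings' PositionsToMove and update neighbour states.
; Its SetColorOver helper sets StateOfTile, checking that array, but applies the same material for every state.
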(event EventBeginPlay
  (bind _returnvalue (Rendering|Material|CreateDynamicMaterialInstance (Variables|Default|GetOver) 0 "/Game/Models/Materials/M_Tile_MaterialMovement.M_Tile_MaterialMovement" :!class /Script/Engine.PrimitiveComponent))
  (Variables|Default|SetDynamicMaterial _returnvalue))

(event EventTick
  (params (DeltaSeconds :type Float%20%28single-precision%29))
  (Utilities|FlowControl|Delay 2.0)
  (Rendering|Material|SetTextureParameterValue (Variables|Default|GetDynamicMaterial) "TextureOverTile" "/Game/_Resources/Images/tile_naranja.tile_naranja")
  (Rendering|SetVisibility (Variables|Default|GetOver) true false))

(event EventActorOnInputTouchEnter
  (params (FingerIndex :type ETouchIndex%20Enum :default "Touch1"))
  (bind _returnvalue (Game|GetPlayerController 0))
  (bind _array (Utilities|Array|MakeArray "ObjectTypeQuery2"))
  (bind _hitresult (Class|PlayerController|GetHitResultUnderFingerforObjects _returnvalue "Touch1" _array true))
  (bind _location (Collision|BreakHitResult _hitresult))
  (bind (_x _y) (Math|Vector|BreakVector _location))
  (Development|PrintString (Utilities|String|ToString(Vector) (Math|Vector|MakeVector _x _y 0.0)) true true "(R=0.034607,G=1.000000,B=0.000000,A=1.000000)" 1e+01))

(event EventActorOnInputTouchBegin
  (params (FingerIndex :type ETouchIndex%20Enum :default "Touch1")))

(fn ConstructionScript)

(fn IsNotinArray
  (params (PositionToCheck :type Vector))
  (bind _asactor_for_testing_things (Utilities|Casting|CastToActorForTestingThings (Variables|Default|GetPositionsArray))
    (:then
      (if (Utilities|Array|ContainsItem (Variables|/Game/BluePrints/ActorForTestingThings.ActorForTestingThings_C|GetPositionsToMove _asactor_for_testing_things) PositionToCheck)
        (return true)
        (else
          (return false))))
    (:CastFailed
      (return false))))

(fn SetColorOver
  (params (State :type Integer) (tiles :type Array%20of%20Actor%20Object%20References))
  (for _array_element tiles
    (bind _astile_bp (Utilities|Casting|CastToTile_BP _array_element))
    (switch int State
      (:1
        (Rendering|Material|SetMaterial (Variables|Tile_BP_C|GetOver _astile_bp) 0 "/Game/Models/Materials/M_Tile_MaterialMovement.M_Tile_MaterialMovement")
        (Variables|Tile_BP_C|SetStateOfTile _astile_bp 1)
        (bind _isinarray (CallFunction|IsNotinArray (Transformation|GetActorLocation _astile_bp)))
        (if _isinarray
          (bind _asactor_for_testing_things (Utilities|Casting|CastToActorForTestingThings (Variables|Default|GetPositionsArray)))
          (if (Utilities|Array|ContainsItem (Variables|/Game/BluePrints/ActorForTestingThings.ActorForTestingThings_C|GetPositionsToMove _asactor_for_testing_things) (Transformation|GetActorLocation _astile_bp))
            (if (Math|Vector|Equal(Vector) (Utilities|Array|Get(acopy) (Variables|/Game/BluePrints/ActorForTestingThings.ActorForTestingThings_C|GetPositionsToMove _asactor_for_testing_things) (Utilities|Array|LastIndex (Variables|/Game/BluePrints/ActorForTestingThings.ActorForTestingThings_C|GetPositionsToMove _asactor_for_testing_things))) (Transformation|GetActorLocation _astile_bp) 0.0)
              (Rendering|Material|SetMaterial (Variables|Tile_BP_C|GetOver _astile_bp) 0 "/Game/Models/Materials/M_Tile_MaterialMovement.M_Tile_MaterialMovement")
              (Variables|Tile_BP_C|SetStateOfTile _astile_bp 4)
              (else
                (Rendering|Material|SetMaterial (Variables|Tile_BP_C|GetOver _astile_bp) 0 "/Game/Models/Materials/M_Tile_MaterialMovement.M_Tile_MaterialMovement")
                (Variables|Tile_BP_C|SetStateOfTile _astile_bp 2))))))
      (:2
        (Rendering|Material|SetMaterial (Variables|Tile_BP_C|GetOver _astile_bp) 0 "/Game/Models/Materials/M_Tile_MaterialMovement.M_Tile_MaterialMovement")
        (Variables|Tile_BP_C|SetStateOfTile _astile_bp 2))
      (:3
        (Rendering|Material|SetMaterial (Variables|Tile_BP_C|GetOver _astile_bp) 0 "/Game/Models/Materials/M_Tile_MaterialMovement.M_Tile_MaterialMovement")
        (Variables|Tile_BP_C|SetStateOfTile _astile_bp 3))
      (:4
        (Rendering|Material|SetMaterial (Variables|Tile_BP_C|GetOver _astile_bp) 0 "/Game/Models/Materials/M_Tile_MaterialMovement.M_Tile_MaterialMovement")
        (Variables|Tile_BP_C|SetStateOfTile _astile_bp 4)))))
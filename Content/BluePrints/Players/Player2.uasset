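; Player2 is a player Blueprint whose Cube component serves as its skin, showing a melee, ranged or magician icon material.
; SetSkinMesh switches on an index to assign the matching material instance to slot 0, and GetMySkinMesh returns the Cube.
; The construction script stores a dynamic material instance of that slot, which SetSkinMesh does not use when swapping materials.
; The event graph holds no logic.
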(event EventBeginPlay)

(event Collision|EventActorBeginOverlap
  (params (OtherActor :type Actor%20Object%20Reference)))

(event EventTick
  (params (DeltaSeconds :type Float%20%28single-precision%29)))

(fn ConstructionScript
  (bind _returnvalue (Rendering|Material|CreateDynamicMaterialInstance (Variables|Default|GetCube) 0 0 :!class /Script/Engine.PrimitiveComponent))
  (Variables|Default|SetMaterialDynamicInstance _returnvalue))

(fn SetSkinMesh
  (params (StaticMeshIndex :type Integer))
  (bind _cube (Variables|Default|GetCube))
  (switch int StaticMeshIndex
    (:0
      (Rendering|Material|SetMaterial _cube 0 "/Game/Models/Characters/Players/M_Icon_melee_Inst.M_Icon_melee_Inst"))
    (:1
      (Rendering|Material|SetMaterial _cube 0 "/Game/Models/Characters/Players/M_Icon_ranged_Inst.M_Icon_ranged_Inst"))
    (:2
      (Rendering|Material|SetMaterial _cube 0 "/Game/Models/Characters/Players/M_Icon_magician_Inst.M_Icon_magician_Inst"))))

(fn GetMySkinMesh
  (return (Variables|Default|GetCube)))
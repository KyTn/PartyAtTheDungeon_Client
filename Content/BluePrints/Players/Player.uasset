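; Player Blueprint with a Cube component whose color can be switched among a fixed palette.
; The construction script creates a dynamic material instance on the cube and stores it.
; ChangeMaterial maps its Color input to a preset by setting the instance's "Color" vector parameter, with black as the fallback.
; The event graph holds no logic.
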(event EventBeginPlay)

(event Collision|EventActorBeginOverlap
  (params (OtherActor :type Actor%20Object%20Reference)))

(event EventTick
  (params (DeltaSeconds :type Float%20%28single-precision%29)))

(fn ConstructionScript
  (bind _returnvalue (Rendering|Material|CreateDynamicMaterialInstance (Variables|Default|GetCube) 0 0 :!class /Script/Engine.PrimitiveComponent))
  (Variables|Default|SetMaterialDynamicInstance _returnvalue))

(fn ChangeMaterial
  (params (Color :type Integer))
  (bind _materialdynamicinstance (Variables|Default|GetMaterialDynamicInstance))
  (bind _materialdynamicinstance_2 (Variables|Default|GetMaterialDynamicInstance))
  (switch int Color
    (:Default
      (Rendering|Material|SetVectorParameterValue (Variables|Default|GetMaterialDynamicInstance) "Color" "(R=0.000000,G=0.000000,B=0.000000,A=1.000000)" :!class /Script/Engine.MaterialInstanceDynamic :!label _label))
    (:0
      (Rendering|Material|SetVectorParameterValue _materialdynamicinstance_2 "Color" "(R=1.000000,G=0.000000,B=0.000000,A=1.000000)" :!class /Script/Engine.MaterialInstanceDynamic))
    (:1
      (Rendering|Material|SetVectorParameterValue _materialdynamicinstance_2 "Color" "(R=0.000000,G=1.000000,B=0.000000,A=1.000000)" :!class /Script/Engine.MaterialInstanceDynamic))
    (:2
      (Rendering|Material|SetVectorParameterValue _materialdynamicinstance_2 "Color" "(R=0.000000,G=0.000000,B=1.000000,A=1.000000)" :!class /Script/Engine.MaterialInstanceDynamic))
    (:3
      (Rendering|Material|SetVectorParameterValue _materialdynamicinstance_2 "Color" "(R=1.000000,G=1.000000,B=0.000000,A=1.000000)" :!class /Script/Engine.MaterialInstanceDynamic))
    (:4
      (Rendering|Material|SetVectorParameterValue _materialdynamicinstance "Color" "(R=1.000000,G=0.000000,B=1.000000,A=1.000000)" :!class /Script/Engine.MaterialInstanceDynamic))
    (:5
      (Rendering|Material|SetVectorParameterValue _materialdynamicinstance "Color" "(R=1.000000,G=0.166000,B=0.000000,A=1.000000)" :!class /Script/Engine.MaterialInstanceDynamic))
    (:6
      (Rendering|Material|SetVectorParameterValue _materialdynamicinstance "Color" "(R=0.000000,G=1.000000,B=1.000000,A=1.000000)" :!class /Script/Engine.MaterialInstanceDynamic))
    (:7
      (Rendering|Material|SetVectorParameterValue _materialdynamicinstance "Color" "(R=1.000000,G=1.000000,B=1.000000,A=1.000000)" :!class /Script/Engine.MaterialInstanceDynamic))
    (:8
      (goto _label))))
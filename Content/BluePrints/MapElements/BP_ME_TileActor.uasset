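; Map tile actor that changes its static mesh material to show move or action highlighting.
; BeginPlay caches the mesh's first material, and three helper functions apply the moving or action highlight or restore that original.
; The event graph's logic reading game-manager status and action type from PD_ClientGameInstance is disconnected, so the actor never calls these helpers itself.
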(event EventBeginPlay
  (bind _asmaterial (Utilities|Casting|CastToMaterial (Rendering|Material|GetMaterial (Variables|Default|GetStaticMesh) 0)))
  (Variables|Default|SetInitialMaterial _asmaterial))

(event EventTick
  (params (DeltaSeconds :type Float%20%28single-precision%29)))

(fn ConstructionScript)

(fn ToOverMovingMaterial
  (Rendering|Material|SetMaterial (Variables|Default|GetStaticMesh) 0 "/Game/Models/Materials/M_Tile_OverMoving.M_Tile_OverMoving"))

(fn ToOverActionMaterial
  (Rendering|Material|SetMaterial (Variables|Default|GetStaticMesh) 0 "/Game/Models/Materials/M_Tile_OverAction.M_Tile_OverAction"))

(fn ResettoInitMaterial
  (Rendering|Material|SetMaterial (Variables|Default|GetStaticMesh) 0 (Variables|Default|GetInitialMaterial)))
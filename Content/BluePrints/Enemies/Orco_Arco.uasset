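; Orco_Arco is an enemy Blueprint that displays its character ID as a name label.
; On BeginPlay it casts the Name component's widget to UI_C_NamePlayer, prints the character ID and writes it to the widget's NameChar.
; An unconnected branch would store the mesh's first material as OriginMaterial before the name setup, but it never runs.
; Tick, overlap and construction logic are empty.
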(event EventBeginPlay
  (bind _asui_c_name_player (Utilities|Casting|CastToUI_C_NamePlayer (UserInterface|GetUserWidgetObject (Variables|Default|GetName))))
  (bind _id_char (Class|PDECharacter|GetCharacterID))
  (Development|PrintString _id_char)
  (Variables|/Game/UserInterface/UI_Client/UI_C_NamePlayer.UI_C_NamePlayer_C|SetName_Char _asui_c_name_player (Utilities|Text|ToText(String) _id_char)))

(event Collision|EventActorBeginOverlap
  (params (OtherActor :type Actor%20Object%20Reference)))

(event EventTick
  (params (DeltaSeconds :type Float%20%28single-precision%29)))

(fn ConstructionScript)
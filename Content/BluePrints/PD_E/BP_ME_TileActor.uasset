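; Map tile actor that shows its map skin and colored movement-state highlights.
; The skin function sets one of five themed fog materials on StaticMesh and keeps a dynamic instance for resetting after move or action material swaps.
; DrawMovementMaterial hides the Over component or swaps its dynamic material's texture among four colors, storing the state.
; Tick is empty, and leftover client game-status selection logic is disconnected.
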(event EventBeginPlay
  (bind _asmaterial (Utilities|Casting|CastToMaterial (Rendering|Material|GetMaterial (Variables|Default|GetStaticMesh) 0)))
  (Variables|Default|SetInitialMaterial _asmaterial)
  (bind _returnvalue (Rendering|Material|CreateDynamicMaterialInstance (Variables|Default|GetOver) 0 "/Game/Models/Materials/M_Tile_MaterialMovement.M_Tile_MaterialMovement" :!class /Script/Engine.PrimitiveComponent))
  (Variables|Default|SetDynamicMaterial _returnvalue))

(event EventTick
  (params (DeltaSeconds :type Float%20%28single-precision%29)))

(fn ConstructionScript
  (bind _returnvalue (Rendering|Material|CreateDynamicMaterialInstance (Variables|Default|GetOver) 0 "/Game/Models/Materials/M_Tile_MaterialMovement.M_Tile_MaterialMovement" :!class /Script/Engine.PrimitiveComponent))
  (Variables|Default|SetDynamicMaterial _returnvalue))

(fn ToOverMovingMaterial
  (Rendering|Material|SetMaterial (Variables|Default|GetStaticMesh) 0 "/Game/Models/Materials/M_Tile_OverMoving.M_Tile_OverMoving"))

(fn ToOverActionMaterial
  (Rendering|Material|SetMaterial (Variables|Default|GetStaticMesh) 0 "/Game/Models/Materials/M_Tile_OverAction.M_Tile_OverAction"))

(fn ResettoInitMaterial
  (Rendering|Material|SetMaterial (Variables|Default|GetStaticMesh) 0 (Variables|Default|GetDynamicTileMaterial)))

(fn DrawMovementMaterial
  (params (StateOfTileForMoving :type Integer))
  (Utilities|IsValid (Variables|Default|GetDynamicMaterial)
    (:Is%20Valid
      (switch int StateOfTileForMoving
        (:0
          (Rendering|SetVisibility (Variables|Default|GetOver) false false)
          (Variables|Default|SetStateTileToMove 0))
        (:1
          (Rendering|Material|SetTextureParameterValue (Variables|Default|GetDynamicMaterial) "TextureOverTile" "/Game/_Resources/Images/tile_azul.tile_azul")
          (Variables|Default|SetStateTileToMove 1)
          (Rendering|SetVisibility (Variables|Default|GetOver) true false))
        (:2
          (Rendering|Material|SetTextureParameterValue (Variables|Default|GetDynamicMaterial) "TextureOverTile" "/Game/_Resources/Images/tile_naranja.tile_naranja")
          (Variables|Default|SetStateTileToMove 2)
          (Rendering|SetVisibility (Variables|Default|GetOver) true false))
        (:3
          (Rendering|Material|SetTextureParameterValue (Variables|Default|GetDynamicMaterial) "TextureOverTile" "/Game/_Resources/Images/tile_rojo.tile_rojo")
          (Variables|Default|SetStateTileToMove 3)
          (Rendering|SetVisibility (Variables|Default|GetOver) true false))
        (:4
          (Rendering|Material|SetTextureParameterValue (Variables|Default|GetDynamicMaterial) "TextureOverTile" "/Game/_Resources/Images/tile_verde.tile_verde")
          (Variables|Default|SetStateTileToMove 4)
          (Rendering|SetVisibility (Variables|Default|GetOver) true false))))
    (:Is%20Not%20Valid
      (Development|PrintString "Material Not Valid" true true "(R=1.000000,G=0.000000,B=0.053811,A=1.000000)"))))

(fn BPChangeMaterialPropertiesMapSkin
  (bind _staticmesh (Variables|Default|GetStaticMesh))
  (bind _returnvalue (Class|PDEElementActor|GetMaterialSkin))
  (switch Utilities|FlowControl|Switch|SwitchonMapSkinType _returnvalue
    (:DUNGEON_NORMAL
      (Rendering|Material|SetMaterial _staticmesh 0 "/Game/Models/PD_E/ESC/SK_DUNG/TILES/M_Dungeon_Tiles_Fog_Inst_01.M_Dungeon_Tiles_Fog_Inst_01")
      (bind _returnvalue_2 (Rendering|Material|CreateDynamicMaterialInstance _staticmesh 0 0 :!class /Script/Engine.PrimitiveComponent))
      (Variables|Default|SetDynamicTileMaterial _returnvalue_2))
    (:GARDEN
      (Rendering|Material|SetMaterial _staticmesh 0 "/Game/Models/PD_E/ESC/SK_GARD/TILES/M_Garden_Tiles_Fog_Inst_01.M_Garden_Tiles_Fog_Inst_01")
      (bind _returnvalue_3 (Rendering|Material|CreateDynamicMaterialInstance _staticmesh 0 0 :!class /Script/Engine.PrimitiveComponent))
      (Variables|Default|SetDynamicTileMaterial _returnvalue_3))
    (:LIBRARY
      (Rendering|Material|SetMaterial _staticmesh 0 "/Game/Models/PD_E/ESC/SK_LIBR/TILES/M_Library_Tiles_Fog_Inst.M_Library_Tiles_Fog_Inst")
      (bind _returnvalue_4 (Rendering|Material|CreateDynamicMaterialInstance _staticmesh 0 0 :!class /Script/Engine.PrimitiveComponent))
      (Variables|Default|SetDynamicTileMaterial _returnvalue_4))
    (:SACRIFICE
      (Rendering|Material|SetMaterial _staticmesh 0 "/Game/Models/PD_E/ESC/SK_SACR/TILES/M_Sacrifice_Tiles_Fog_Inst.M_Sacrifice_Tiles_Fog_Inst")
      (bind _returnvalue_5 (Rendering|Material|CreateDynamicMaterialInstance _staticmesh 0 0 :!class /Script/Engine.PrimitiveComponent))
      (Variables|Default|SetDynamicTileMaterial _returnvalue_5))
    (:BOSS
      (Rendering|Material|SetMaterial _staticmesh 0 "/Game/Models/PD_E/ESC/SK_BOSS/TILES/M_Boss_Tiles_Fog_Inst.M_Boss_Tiles_Fog_Inst")
      (bind _returnvalue_6 (Rendering|Material|CreateDynamicMaterialInstance _staticmesh 0 0 :!class /Script/Engine.PrimitiveComponent))
      (Variables|Default|SetDynamicTileMaterial _returnvalue_6))))
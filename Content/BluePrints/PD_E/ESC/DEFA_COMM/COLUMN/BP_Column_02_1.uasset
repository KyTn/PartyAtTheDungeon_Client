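; Column prop Blueprint that re-skins its mesh to match the map's theme.
; BP_ChangeMaterialProperties_MapSkin switches on GetMaterialSkin and sets material slot 0, picking randomly among three fog tile variants for Dungeon, Garden and Sacrifice.
; Library and Boss use fixed materials wrapped in dynamic instances, though Boss builds its instance from the Prop fog material, replacing the Tiles one just set.
; The event graph and construction script are empty.
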(event EventBeginPlay)

(event Collision|EventActorBeginOverlap
  (params (OtherActor :type Actor%20Object%20Reference)))

(event EventTick
  (params (DeltaSeconds :type Float%20%28single-precision%29)))

(fn ConstructionScript)

(fn BPChangeMaterialPropertiesMapSkin
  (bind _mesh (Variables|Default|Getmesh))
  (bind _returnvalue (Class|PDEElementActor|GetMaterialSkin))
  (switch Utilities|FlowControl|Switch|SwitchonMapSkinType _returnvalue
    (:DUNGEON_NORMAL
      ;[1 1 1] SK_DUNG
      (switch int (Math|Random|RandomIntegerinRange 0 2)
        (:0
          (Rendering|Material|SetMaterial _mesh 0 "/Game/Models/PD_E/ESC/SK_DUNG/TILES/M_Dungeon_Tiles_Fog_Inst_01.M_Dungeon_Tiles_Fog_Inst_01"))
        (:1
          (Rendering|Material|SetMaterial _mesh 0 "/Game/Models/PD_E/ESC/SK_DUNG/TILES/M_Dungeon_Tiles_Fog_Inst_02.M_Dungeon_Tiles_Fog_Inst_02"))
        (:2
          (Rendering|Material|SetMaterial _mesh 0 "/Game/Models/PD_E/ESC/SK_DUNG/TILES/M_Dungeon_Tiles_Fog_Inst_03.M_Dungeon_Tiles_Fog_Inst_03"))))
    (:GARDEN
      ;[1 1 1] SK_GARD
      (switch int (Math|Random|RandomIntegerinRange 0 2)
        (:0
          (Rendering|Material|SetMaterial _mesh 0 "/Game/Models/PD_E/ESC/SK_GARD/TILES/M_Garden_Tiles_Fog_Inst_01.M_Garden_Tiles_Fog_Inst_01"))
        (:1
          (Rendering|Material|SetMaterial _mesh 0 "/Game/Models/PD_E/ESC/SK_GARD/TILES/M_Garden_Tiles_Fog_Inst_02.M_Garden_Tiles_Fog_Inst_02"))
        (:2
          (Rendering|Material|SetMaterial _mesh 0 "/Game/Models/PD_E/ESC/SK_GARD/TILES/M_Garden_Tiles_Fog_Inst_03.M_Garden_Tiles_Fog_Inst_03"))))
    (:LIBRARY
      (Rendering|Material|SetMaterial _mesh 0 "/Game/Models/PD_E/ESC/SK_LIBR/TILES/M_Library_Tiles_Fog_Inst.M_Library_Tiles_Fog_Inst")
      (Rendering|Material|CreateDynamicMaterialInstance _mesh 0 "/Game/Models/PD_E/ESC/SK_LIBR/TILES/M_Library_Tiles_Fog_Inst.M_Library_Tiles_Fog_Inst" :!class /Script/Engine.PrimitiveComponent))
    (:SACRIFICE
      ;[1 1 1] SK_SACR
      (switch int (Math|Random|RandomIntegerinRange 0 2)
        (:0
          (Rendering|Material|SetMaterial _mesh 0 "/Game/Models/PD_E/ESC/SK_SACR/TILES/M_Sacrifice_Tiles_Fog_Inst_01.M_Sacrifice_Tiles_Fog_Inst_01"))
        (:1
          (Rendering|Material|SetMaterial _mesh 0 "/Game/Models/PD_E/ESC/SK_SACR/TILES/M_Sacrifice_Tiles_Fog_Inst_02.M_Sacrifice_Tiles_Fog_Inst_02"))
        (:2
          (Rendering|Material|SetMaterial _mesh 0 "/Game/Models/PD_E/ESC/SK_SACR/TILES/M_Sacrifice_Tiles_Fog_Inst_03.M_Sacrifice_Tiles_Fog_Inst_03"))))
    (:BOSS
      (Rendering|Material|SetMaterial _mesh 0 "/Game/Models/PD_E/ESC/SK_BOSS/TILES/M_Boss_Tiles_Fog_Inst.M_Boss_Tiles_Fog_Inst")
      (Rendering|Material|CreateDynamicMaterialInstance _mesh 0 "/Game/Models/PD_E/ESC/SK_BOSS/PROPS/M_Boss_Prop_Fog_Inst.M_Boss_Prop_Fog_Inst" :!class /Script/Engine.PrimitiveComponent))))